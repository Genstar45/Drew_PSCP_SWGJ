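; BP_Prop is a billboard prop whose static mesh turns to face the player camera, as for a sprite.
; The construction script applies the Mat material to the mesh's first slot.
; Each Tick sets the mesh's world yaw to the camera yaw plus a 90-degree offset, with pitch and roll held at zero so it stays upright.
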(event EventTick
  (params (DeltaSeconds :type Float%20%28single-precision%29))
  (bind _staticmesh (Variables|Default|GetStaticMesh))
  ;[1 1 1] player sprite faces camera
  (Utilities|IsValid _staticmesh
    (:Is%20Valid
      (Transformation|SetWorldRotation _staticmesh (Math|Rotator|MakeRotator 0.0 0.0 (+ 9e+01 (.yaw (Camera|GetCameraRotation (Game|GetPlayerCameraManager 0))))) false false))))

(fn ConstructionScript
  (Rendering|Material|SetMaterial (Variables|Default|GetStaticMesh) 0 (Variables|Default|Getmat)))