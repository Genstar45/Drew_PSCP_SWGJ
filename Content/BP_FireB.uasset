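; BP_FireB is a moving fire hazard that kills BP_TopDownCharacter on overlap.
; After a configurable start delay, Loop and AddUp cycle a counter that drives MoveComponentTo, carrying the sprite around four waypoint components in one-second legs.
; Tick line-traces downward to place the drop shadow on the surface below and billboards the sprite toward the player camera.
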(event Custom|Loop
  (bind _1 (Variables|Default|Get1))
  (bind _sprite (Variables|Default|GetSprite))
  (bind _rotation (Variables|Default|Getrotation))
  (bind _relativelocation (Variables|/Script/Engine.SceneComponent|GetRelativeLocation _1))
  (switch int (Variables|Default|Getnumber)
    (:0
      (bind _output_get (Variables|Default|SetstartPos _relativelocation))
      (Variables|Default|Setnumber 1)
      (Components|MoveComponentTo (Variables|Default|GetSprite) _output_get "0, 0, 0" false false 0.0 false)
      (CallFunction|Loop))
    (:1
      (bind _output_get_2 (Variables|Default|SetendPos (Variables|/Script/Engine.SceneComponent|GetRelativeLocation (Variables|Default|Get2))))
      (Components|MoveComponentTo _sprite _output_get_2 _rotation false false 1.0 false)
      (CallFunction|AddUp))
    (:2
      (bind _output_get_3 (Variables|Default|SetendPos (Variables|/Script/Engine.SceneComponent|GetRelativeLocation (Variables|Default|Get3))))
      (Components|MoveComponentTo _sprite _output_get_3 _rotation false false 1.0 false)
      (CallFunction|AddUp))
    (:3
      (bind _output_get_4 (Variables|Default|SetendPos (Variables|/Script/Engine.SceneComponent|GetRelativeLocation (Variables|Default|Get4))))
      (Components|MoveComponentTo _sprite _output_get_4 _rotation false false 1.0 false)
      (CallFunction|AddUp))
    (:4
      (bind _output_get_5 (Variables|Default|SetendPos _relativelocation))
      (Components|MoveComponentTo _sprite _output_get_5 _rotation false false 1.0 false)
      (CallFunction|AddUp))))

(event Custom|AddUp
  (Variables|Default|SetstartPos (Variables|Default|GetendPos))
  (bind _output_get (Variables|Default|Setnumber (+ (Variables|Default|Getnumber) 1)))
  (if (> _output_get 4)
    (Variables|Default|Setnumber 0))
  (CallFunction|Loop))

(event EventTick
  (params (DeltaSeconds :type Float%20%28single-precision%29))
  (bind _returnvalue (Game|GetPlayerCameraManager 0))
  (bind _sprite (Variables|Default|GetSprite))
  (bind _returnvalue_2 (Transformation|GetWorldLocation _sprite))
  (bind _returnvalue_3 (Camera|GetCameraRotation _returnvalue))
  (Utilities|FlowControl|Sequence
    (:then_0
      ;[1 1 1] drop shadow
      (bind _outhit (Collision|LineTraceByChannel (Math|Vector|MakeVector (.x _returnvalue_2) (.y _returnvalue_2) (+ (.z _returnvalue_2) 1e+01)) (Math|Vector|MakeVector (.x _returnvalue_2) (.y _returnvalue_2) -1e+03) "TraceTypeQuery1" false 0 "None" true "(R=0.000000,G=0.000000,B=0.000000,A=0.800000)" "(R=0.000000,G=0.000000,B=0.000000,A=0.634783)"))
      (Transformation|SetRelativeLocation (Variables|Default|GetDropShadow) (Math|Vector|MakeVector (.x (.ImpactPoint (Collision|BreakHitResult _outhit))) (.y (.ImpactPoint (Collision|BreakHitResult _outhit))) (+ (.z (.ImpactPoint (Collision|BreakHitResult _outhit))) 1.0)) false false))
    (:then_1
      ;[1 1 1] player sprite faces camera
      (Utilities|IsValid (Variables|Default|GetSprite)
        (:Is%20Valid
          (bind _output_get (Variables|Default|Setrotation (Math|Rotator|MakeRotator (.pitch _returnvalue_3) 0.0 (+ 9e+01 (.yaw _returnvalue_3)))))
          (Transformation|SetWorldRotation (Variables|Default|GetSprite) _output_get false false))))))

(event Collision|EventActorBeginOverlap
  (params (OtherActor :type Actor%20Object%20Reference))
  (bind _asbp_top_down_character (Utilities|Casting|CastToBP_TopDownCharacter OtherActor))
  (Default|Die _asbp_top_down_character))

(event EventBeginPlay
  (Utilities|FlowControl|Delay (Variables|Default|GetwaitBeforeStart))
  (CallFunction|Loop))

(fn ConstructionScript)