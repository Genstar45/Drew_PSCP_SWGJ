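; BP_Collectible is a gem pickup that notifies BP_TopDownCharacter through OnGemCollect on overlap, then destroys itself.
; Each tick, a downward Visibility trace positions its DropShadow just above the impact point, passing that world-space point to SetRelativeLocation.
; Tick also billboards the PaperFlipbook sprite, deriving its roll from camera pitch and its yaw from camera yaw offset by a quarter turn.
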(event EventTick
  (params (DeltaSeconds :type Float%20%28single-precision%29))
  (bind _returnvalue (Transformation|GetActorLocation))
  (bind _returnvalue_2 (Game|GetPlayerCameraManager 0))
  (bind _returnvalue_3 (Camera|GetCameraRotation _returnvalue_2))
  (Utilities|FlowControl|Sequence
    (:then_0
      ;[1 1 1] drop shadow
      (bind _outhit (Collision|LineTraceByChannel (Math|Vector|MakeVector (.x _returnvalue) (.y _returnvalue) (+ (.z _returnvalue) 1e+01)) (Math|Vector|MakeVector (.x _returnvalue) (.y _returnvalue) -1e+03) "TraceTypeQuery1" false 0 "None" true "(R=0.000000,G=0.000000,B=0.000000,A=0.800000)" "(R=0.000000,G=0.000000,B=0.000000,A=0.634783)"))
      (Transformation|SetRelativeLocation (Variables|Default|GetDropShadow) (Math|Vector|MakeVector (.x (.ImpactPoint (Collision|BreakHitResult _outhit))) (.y (.ImpactPoint (Collision|BreakHitResult _outhit))) (+ (.z (.ImpactPoint (Collision|BreakHitResult _outhit))) 1.0)) false false))
    (:then_1
      ;[1 1 1] player sprite faces camera
      (Utilities|IsValid (Variables|Default|GetPaperFlipbook)
        (:Is%20Valid
          (Transformation|SetWorldRotation (Variables|Default|GetPaperFlipbook) (Math|Rotator|MakeRotator (.pitch _returnvalue_3) 0.0 (+ 9e+01 (.yaw _returnvalue_3))) false false))))))

(event Collision|EventActorBeginOverlap
  (params (OtherActor :type Actor%20Object%20Reference))
  (bind _asbp_top_down_character (Utilities|Casting|CastToBP_TopDownCharacter OtherActor))
  (Default|OnGemCollect _asbp_top_down_character)
  (Actor|DestroyActor))

(fn ConstructionScript)