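; Stretchable actor that grows along Z by a Value passed to ChangeScaleZ, limited by obstacles above it.
; BeginPlay stores the original transform and, after a short delay, caches a Slider_Widget reference.
; ChangeScaleZ box-traces upward to cap the stretch at the hit distance or OgMax.
; A Timeline then lerps the actor's scale while overriding the planes' world scale and spinning the arrow.
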(event Custom|ChangeScaleZ
  (params (value :type Float%20%28double-precision%29))
  (bind _ogsize (Variables|Default|GetogSize))
  (bind _ogsize_2 (Variables|Default|GetogSize))
  (bind _arrow (Variables|Default|GetArrow))
  (bind _returnvalue (* _ogsize_2 50))
  (bind _relativerotation (Variables|/Script/Engine.SceneComponent|GetRelativeRotation _arrow))
  (bind (_outhit _returnvalue_2) (Collision|BoxTraceByChannel (Variables|Default|GetrayStartPos) (+ (Variables|Default|GetrayStartPos) (Math|Vector|MakeVector 0.0 0.0 (* (Variables|Default|GetogMax) 1e+02))) (Math|Vector|MakeVector (- (.x _returnvalue) 1.0) (- (.y _returnvalue) 1.0) 0.0) "0, 0, 0" "TraceTypeQuery1" false 0 "ForOneFrame" true "(R=0.000000,G=0.000000,B=1.000000,A=1.000000)" "(R=1.000000,G=0.000000,B=0.767453,A=1.000000)"))
  (if _returnvalue_2
    (Variables|Default|SetcurrentMax (/ (.Distance (Collision|BreakHitResult _outhit)) 1e+02))
    (bind _newtrack_0 (Timeline|Timeline PlayFromStart)
      (:Update
        (Transformation|SetActorScale3D (Math|Vector|Lerp(Vector) (Transformation|GetActorScale3D) (Math|Vector|MakeVector (.x _ogsize) (.y _ogsize) (+ (.z _ogsize) (* (Variables|Default|GetcurrentMax) value))) _newtrack_0))
        (Transformation|SetWorldScale3D (Variables|Default|GetPlane) (Math|Vector|MakeVector 1.0 1.0 1.0))
        (Transformation|SetWorldScale3D (Variables|Default|GetPlane2) (Math|Vector|MakeVector 1.0 1.0 (.Z (Math|Vector|BreakVector (Math|Vector|Lerp(Vector) (Transformation|GetActorScale3D) (Math|Vector|MakeVector (.x _ogsize) (.y _ogsize) (+ (.z _ogsize) (* (Variables|Default|GetcurrentMax) value))) _newtrack_0)))))
        (Transformation|SetWorldScale3D (Variables|Default|GetPlane1) (Math|Vector|MakeVector 1.0 1.0 (.Z (Math|Vector|BreakVector (Math|Vector|Lerp(Vector) (Transformation|GetActorScale3D) (Math|Vector|MakeVector (.x _ogsize) (.y _ogsize) (+ (.z _ogsize) (* (Variables|Default|GetcurrentMax) value))) _newtrack_0)))))
        (Transformation|SetRelativeRotation _arrow (Math|Rotator|MakeRotator (.roll _relativerotation) (.pitch _relativerotation) (+ (.yaw _relativerotation) 3.0)) false false)))
    (else
      (Variables|Default|SetcurrentMax (Variables|Default|GetogMax))
      (Timeline|Timeline PlayFromStart))))

(event EventBeginPlay
  (Utilities|FlowControl|Sequence
    (:then_0
      (Variables|Default|SetogSize (Transformation|GetActorScale3D))
      (Variables|Default|SetogPos (Transformation|GetActorLocation))
      (Variables|Default|SetcurrentMax (Variables|Default|GetogMax))
      (Variables|Default|SetrayStartPos (+ (Variables|Default|GetogPos) (Math|Vector|MakeVector (.x (* (Variables|Default|GetogSize) 50)) (.y (* (Variables|Default|GetogSize) 50)) (* 2.0 (.z (* (Variables|Default|GetogSize) 50)))))))
    (:then_1
      (Utilities|FlowControl|Delay 0.5)
      (bind _foundwidgets (Widget|GetAllWidgetsOfClass "/Game/Slider_Widget.Slider_Widget_C" false))
      (Variables|Default|SetwidgetReference (Utilities|Array|Get(acopy) _foundwidgets)))))

(fn ConstructionScript)